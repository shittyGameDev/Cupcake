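; BP_TreeWeapon is an item actor that knocks the player back when a BP_PlayerCharacter overlaps it.
; On overlap it disables character movement and briefly turns the capsule into a plane-constrained physics body, launched by a fixed-direction velocity-change impulse.
; After a short delay it switches physics off, clears the constraint and restores walking.
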(event `self.ReceiveActorBeginOverlap`
  (params (OtherActor :type "Actor Object Reference"))
  (bind _player (`self.Player`))
  (bind _asbp_player_character (cast `/Game/Player/BP_PlayerCharacter` OtherActor))
  (bind _output_get (set `self.Player` _asbp_player_character))
  (`CharacterMovementComponent.SetMovementMode` (`Character.CharacterMovement` _output_get) "MOVE_None" 0)
  (bind _capsulecomponent (`Character.CapsuleComponent` _output_get))
  (`PrimitiveComponent.SetConstraintMode` _capsulecomponent "XYPlane")
  (`PrimitiveComponent.SetSimulatePhysics` _capsulecomponent true)
  (`PrimitiveComponent.AddImpulse` _capsulecomponent (200.0 200.0 10.0) "None" true)
  (`KismetSystemLibrary.Delay` 1.0)
  (`PrimitiveComponent.SetSimulatePhysics` (`Character.CapsuleComponent` _player) false)
  (`PrimitiveComponent.SetConstraintMode` _capsulecomponent "None")
  (`CharacterMovementComponent.SetMovementMode` (`Character.CharacterMovement` _player) "MOVE_Walking" 0))

(fn `UserConstructionScript`)