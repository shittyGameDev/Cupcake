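; Mushroom enemy character in the gang AI system, with a charge-then-launch attack, hurt sound and death handling.
; StartAttack chains charge and attack montages, whose notifies play audio events and equip or unequip the weapon for the hit window.
; OnDeath stops movement, plays the death montage and drops an item for the player.
; When that montage ends, it unregisters from GangAIManager and, if the weapon is valid, destroys weapon and self.
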(event `self.StartAttack`
  (bind _weapon (`self.Weapon`))
  (bind _mesh (`self.Mesh`))
  (bind _returnvalue (`KismetMathLibrary.Conv_VectorToTransform` (`self.K2_GetActorLocation` self)))
  (bind _notifyname (`|PlayMontage` _mesh "/Game/Blueprints/Enemies/Mushroom/Animations/MushroomCharge_Montage.MushroomCharge_Montage")
    (:`OnCompleted`
      (bind _notifyname_2 (`|PlayMontage` _mesh "/Game/Blueprints/Enemies/Mushroom/Animations/MushroomAttack_Montage.MushroomAttack_Montage")
        (:`OnNotifyBegin`
          (switch `name` _notifyname_2
            (:`Launch`
              (`FMODBlueprintStatics.PlayEventAtLocation` "/Game/FMOD/Events/Mushroom_Enemy/MushroomLaunch.MushroomLaunch" _returnvalue))
            (:`Hit`
              (`WeaponBase.Equip` _weapon))
            (:`FHit`
              (`WeaponBase.Unequip` _weapon))
            (:`Land`
              (`FMODBlueprintStatics.PlayEventAtLocation` "/Game/FMOD/Events/Mushroom_Enemy/MushroomLand.MushroomLand" _returnvalue))))))
    (:`OnNotifyBegin`
      (switch `name` _notifyname
        (:`Charge`
          (`FMODBlueprintStatics.PlayEventAtLocation` "/Game/FMOD/Events/Mushroom_Enemy/MushroomCharge.MushroomCharge" _returnvalue))))))

(event `self.ReceiveBeginPlay`
  (`AttributeComponent.SetMaxHealth` (`self.GetComponentByClass` self "/Script/Cupcake.AttributeComponent") 100.0))

(event `self.PlayHurtSound`
  (`FMODBlueprintStatics.PlayEventAtLocation` "/Game/FMOD/Events/Mushroom_Enemy/MushroomLand.MushroomLand" (`KismetMathLibrary.Conv_VectorToTransform` (`self.K2_GetActorLocation` self))))

(event `DamageableInterface.OnDeath`
  (bind _weapon (`self.Weapon`))
  (`CharacterMovementComponent.SetMovementMode` (`self.CharacterMovement`) "MOVE_None" 0)
  (bind _notifyname (`|PlayMontage` (`self.Mesh`) "/Game/Blueprints/Enemies/Mushroom/Animations/MushroomDeath_Montage.MushroomDeath_Montage")
    (:`then`
      (bind _ascupcake_character (cast `CupcakeCharacter` (`GameplayStatics.GetPlayerCharacter` 0)))
      (`DropComponent.DropItem` (`self.Drop`) _ascupcake_character)
      (`KismetSystemLibrary.PrintString` "William älskar genshin impact så mycket att han tar av sig byxorna")
      (`KismetSystemLibrary.PrintString` "Hello"))
    (:`OnCompleted`
      (bind _returnvalue (`GameplayStatics.GetActorOfClass` "/Script/Cupcake.GangAIManager" :!label _label))
      (`KismetArrayLibrary.Array_RemoveItem` (`GangAIManager.RegisteredAICharacters` _returnvalue) self)
      (`/Engine/EditorBlueprintResources/StandardMacros.IsValid` _weapon
        (:`Is Valid`
          (`self.K2_DestroyActor` _weapon)
          (`self.K2_DestroyActor`))))
    (:`OnBlendOut`
      (goto _label))
    (:`OnInterrupted`
      (goto _label))
    (:`OnNotifyBegin`
      (switch `name` _notifyname
        (:`Death`
          (`FMODBlueprintStatics.PlayEventAtLocation` "/Game/FMOD/Events/Mushroom_Enemy/MushroomDeath.MushroomDeath" (`KismetMathLibrary.Conv_VectorToTransform` (`self.K2_GetActorLocation` self))))))))

(fn `Random Vector`
  (params (Min :type "Float (double-precision)") (Max :type "Float (double-precision)"))
  (returns (`Return Value` :type "Vector Structure"))
  (return (`KismetMathLibrary.MakeVector` (`KismetMathLibrary.RandomFloatInRange` Min Max) (`KismetMathLibrary.RandomFloatInRange` Min Max))))

(fn `UserConstructionScript`)