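; BP_BaseHUD is a HUD Blueprint that handles animated opening and closing of the main menu and interaction widgets.
; Menu events play open or close animations on the main menu's inventory panel, while interaction events animate the interaction widget itself.
; Opening makes the widget visible as its animation starts, while closing waits a fixed delay for the animation before collapsing the widget.
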(event `self.AnimateOpenMenu`
  (bind _mainmenuwidget (`self.MainMenuWidget`))
  (`Widget.SetVisibility` _mainmenuwidget "Visible")
  (bind _aswbp_inventory_panel (cast `/Game/Blueprints/UI/ImprovedUI/WBP_InventoryPanel` (`MainMenu.InventoryPanel` _mainmenuwidget))
    (:`then`
      (`/Game/Blueprints/UI/ImprovedUI/WBP_InventoryPanel.PlayOpen` _aswbp_inventory_panel))
    (:`CastFailed`
      (`KismetSystemLibrary.PrintString` "Cast failed"))))

(event `self.AnimateCloseMenu`
  (bind _mainmenuwidget (`self.MainMenuWidget`))
  (bind _aswbp_inventory_panel (cast `/Game/Blueprints/UI/ImprovedUI/WBP_InventoryPanel` (`MainMenu.InventoryPanel` _mainmenuwidget))
    (:`then`
      (`/Game/Blueprints/UI/ImprovedUI/WBP_InventoryPanel.PlayClose` _aswbp_inventory_panel)
      (`KismetSystemLibrary.Delay` 0.41)
      (`Widget.SetVisibility` _mainmenuwidget "Collapsed"))
    (:`CastFailed`
      (`KismetSystemLibrary.PrintString` "Cast failed"))))

(event `self.AnimateCloseInteractionWidget`
  (bind _interactionwidget (`self.InteractionWidget`))
  (bind _aswbp_interaction_widget (cast `/Game/Blueprints/UI/ImprovedUI/WBP_InteractionWidget` _interactionwidget))
  (`/Game/Blueprints/UI/ImprovedUI/WBP_InteractionWidget.Animate Close` _aswbp_interaction_widget)
  (`KismetSystemLibrary.Delay` 0.35)
  (`Widget.SetVisibility` _interactionwidget "Collapsed"))

(event `self.AnimateOpenInteractionWidget`
  (bind _aswbp_interaction_widget (cast `/Game/Blueprints/UI/ImprovedUI/WBP_InteractionWidget` (`self.InteractionWidget`)))
  (`Widget.SetVisibility` _aswbp_interaction_widget "Visible")
  (`/Game/Blueprints/UI/ImprovedUI/WBP_InteractionWidget.Animate Open` _aswbp_interaction_widget))

(fn `UserConstructionScript`)