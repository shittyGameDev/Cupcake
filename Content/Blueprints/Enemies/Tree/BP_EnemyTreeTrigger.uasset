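; Tree enemy character that attacks, drops loot on death and triggers other trees to move.
; Swipe runs a sweep attack; swing attacks, plays a montage and signals attack end.
; Death sets IsDead, so Tick tips the actor over along FallCurve, while a macro loop scatters pickups around it before delayed destruction.
; Death also calls MoveTree on every entry in the MoveTree array.
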(event `SwipeAttack`
  (`self.DoSweepAttack`))

(event `self.ReceiveBeginPlay`)

(event `SwingAttack`
  ;[1 1 1] Swing Attack
  (`self.DoAttack`)
  (`|PlayMontage` (`self.Mesh`) "/Game/Animations/Montage_Run.Montage_Run"
    (:`then`
      (`KismetSystemLibrary.Delay` 1.0))
    (:`OnCompleted`
      _)
    (:`OnInterrupted`
      _))
  (`self.OnAttackEnd`))

(event `self.ReceiveTick`
  (params (DeltaSeconds :type "Float (single-precision)"))
  ;[1 1 1] Fall Animation
  (if (`self.IsDead`)
    (set `self.In Time` (+ (`self.In Time`) 0.01))
    (`self.K2_SetActorRotation` (`KismetMathLibrary.RLerp` (`self.GetBaseRotationOffsetRotator`) (struct :`Roll` 70.0) (`CurveFloat.GetFloatValue` (`self.Fall Curve`) (`self.In Time`))))))

(event `DamageableInterface.OnDamage`
  ;[1 1 1] On Damage
  (if (`self.IsDead`)
    _))

(event `DamageableInterface.OnDeath`
  ;[1 1 1] Drop Loot
  (`|ExecutionSequence`
    (:`then_0`
      (set `self.IsDead` true)
      (`KismetSystemLibrary.Delay` 0.2)
      (while (< (`self.Counter`) (`KismetMathLibrary.RandomInteger` (`self.LootAmount`))) :!label _label
        (`|SpawnActorFromClass` "/Game/Blueprints/ItemFolder/PickupBase.PickupBase_C" (`KismetMathLibrary.Conv_VectorToTransform` (+ (.location (`self.GetTransform`)) (`self.Random Vector` -200.0 200.0))) "Undefined" "MultiplyWithRoot" null null)
        (set `self.Counter` (+ 1 (`self.Counter`)))
        (goto _label))
      (`KismetSystemLibrary.Delay` 2.0)
      (`self.K2_DestroyActor`))
    (:`then_1`
      (for _array_element (`self.MoveTree`)
        (`/Game/Blueprints/BP_TutorialTreeMove.MoveTree` _array_element)))))

(fn `Random Vector`
  (params (Min :type "Float (double-precision)") (Max :type "Float (double-precision)"))
  (returns (`Return Value` :type "Vector Structure"))
  (return (`KismetMathLibrary.MakeVector` (`KismetMathLibrary.RandomFloatInRange` Min Max) (`KismetMathLibrary.RandomFloatInRange` Min Max))))

(fn `SetMovementSpeed`
  (params (Speed :type "/Game/Blueprints/Enemies/Tree/AI/Enums/E_MovementSpeed Enum" :default "NewEnumerator0"))
  (returns (SpeedValue :type "Float (double-precision)"))
  (bind _output_get (set `CharacterMovementComponent.MaxWalkSpeed` (select `/Game/Blueprints/Enemies/Tree/AI/Enums/E_MovementSpeed` Speed :`NewEnumerator1` 70.0 :`NewEnumerator2` 150.0 :`NewEnumerator3` 300.0 :!type "Float (single-precision)") (`self.CharacterMovement`)))
  (return _output_get))

(fn `UserConstructionScript`)