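; BP_Map is a world actor that shows a map widget while the player stands inside its collider.
; On BeginPlay it creates WBP_TheMap, adds it to the viewport and hides it.
; Collider overlap events cast to BP_PlayerCharacter, showing the widget on entry and hiding it on exit.
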(event `self.ReceiveBeginPlay`
  (bind _returnvalue (`|CreateWidget` "/Game/Blueprints/UI/WBP_TheMap.WBP_TheMap_C"))
  (bind _output_get (set `self.The Map` _returnvalue))
  (`UserWidget.AddToViewport` _output_get 0)
  (`Widget.SetVisibility` _output_get "Hidden"))

(event `self.collider.OnComponentBeginOverlap`
  (params (OverlappedComponent :type "PrimitiveComponent Object Reference") (OtherActor :type "Actor Object Reference") (OtherComp :type "PrimitiveComponent Object Reference") (OtherBodyIndex :type Integer) (bFromSweep :type Boolean) (SweepResult :type "HitResult Structure (by ref)"))
  (cast `/Game/Blueprints/BP_PlayerCharacter` OtherActor
    (:`then`
      (`Widget.SetVisibility` (`self.The Map`) "Visible"))
    (:`CastFailed`
      (`KismetSystemLibrary.PrintString` "failed to cast"))))

(event `self.collider.OnComponentEndOverlap`
  (params (OverlappedComponent :type "PrimitiveComponent Object Reference") (OtherActor :type "Actor Object Reference") (OtherComp :type "PrimitiveComponent Object Reference") (OtherBodyIndex :type Integer))
  (cast `/Game/Blueprints/BP_PlayerCharacter` OtherActor)
  (`Widget.SetVisibility` (`self.The Map`) "Hidden"))

(fn `UserConstructionScript`)