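; Tutorial tree actor that travels along the spline of a referenced tree track, starting shortly after BeginPlay when active.
; A timeline, rate-scaled by Duration and started at TreeStartOffset, maps its alpha to distance along the spline.
; Each update sets world location and spline rotation, with yaw turned 90 degrees.
; At the end it either restarts from the same offset when looping or destroys itself.
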(event `self.ReceiveBeginPlay`
  (if (`self.IsActive`)
    (`KismetSystemLibrary.Delay` 0.75)
    (`self.MoveTree`)))

(event `MoveTree`
  (bind _returnvalue (`KismetMathLibrary.Lerp` 0.0 (`SplineComponent.GetSplineLength` (`/Game/Blueprints/BP_SplineTrack.TreeCurveMovement` (`self.TreeTrackRef`))) (`self.Alpha`)))
  (`TimelineComponent.SetPlayRate` (`self.TreeMover`) (/ 1.0 (`self.Duration`)) :!label _label)
  (`TimelineComponent.SetNewTime` (`self.TreeMover`) (`self.TreeStartOffset`))
  (bind (_direction _alpha) (`Timeline|TreeMover`)
    (:`Update`
      (set `self.Alpha` _alpha)
      (`self.K2_SetActorLocationAndRotation` (`SplineComponent.GetLocationAtDistanceAlongSpline` (`/Game/Blueprints/BP_SplineTrack.TreeCurveMovement` (`self.TreeTrackRef`)) _returnvalue "World") (`KismetMathLibrary.MakeRotator` (.roll (`SplineComponent.GetRotationAtDistanceAlongSpline` (`/Game/Blueprints/BP_SplineTrack.TreeCurveMovement` (`self.TreeTrackRef`)) _returnvalue "World")) (.pitch (`SplineComponent.GetRotationAtDistanceAlongSpline` (`/Game/Blueprints/BP_SplineTrack.TreeCurveMovement` (`self.TreeTrackRef`)) _returnvalue "World")) (+ 90.0 (.yaw (`SplineComponent.GetRotationAtDistanceAlongSpline` (`/Game/Blueprints/BP_SplineTrack.TreeCurveMovement` (`self.TreeTrackRef`)) _returnvalue "World"))))))
    (:`Finished`
      (if (`self.IsLooping`)
        (goto _label)
        (else
          (`self.K2_DestroyActor`))))))

(fn `UserConstructionScript`)