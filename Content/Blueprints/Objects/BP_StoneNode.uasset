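; BP_StoneNode is a stone resource node that scatters stone pickups when it dies, then destroys itself.
; OnDeath runs a custom while-loop macro that spawns PickupStone actors at random horizontal offsets around the node and increments a counter.
; The loop condition comes from a helper macro meant to compare that counter to a random integer derived from LootAmount.
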(event `DamageableInterface.OnDeath`
  (while (< (`self.Counter`) (`KismetMathLibrary.RandomInteger` (`self.Loot Amount`))) :!label _label
    (`|SpawnActorFromClass` "/Game/Blueprints/ItemFolder/PickupStone.PickupStone_C" (`KismetMathLibrary.Conv_VectorToTransform` (+ (.location (`self.GetTransform`)) (`self.Random Vector` -200.0 200.0))) "Undefined" "MultiplyWithRoot" null null)
    (set `self.Counter` (+ 1 (`self.Counter`)))
    (goto _label))
  (`KismetSystemLibrary.PrintString` "Done")
  (`self.K2_DestroyActor`))

(fn `Random Vector`
  (params (Min :type "Float (double-precision)") (Max :type "Float (double-precision)"))
  (returns (`Return Value` :type "Vector Structure"))
  (return (`KismetMathLibrary.MakeVector` (`KismetMathLibrary.RandomFloatInRange` Min Max) (`KismetMathLibrary.RandomFloatInRange` Min Max))))

(fn `UserConstructionScript`)