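; Player character Blueprint that handles NPC dialogue, melee attacks, hurt reactions and respawning.
; The Speaking input sphere-traces down from a scene component for a BC_Dialogue actor, freezing movement while speech shows in the HUD widget.
; Attacks and hurts play animations directly on the mesh, then restore the Animation Blueprint after fixed delays.
; Death moves the player to the BP_DayCycleManager spawn location and resets max health.
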(event `self.ReceiveBeginPlay`
  (`parent.ReceiveBeginPlay`)
  (bind _returnvalue (`|CreateWidget` "/Game/Blueprints/Dialouge/BP_PlayerDialogue.BP_PlayerDialogue_C"))
  (bind _output_get (set `self.PlayerHUD` _returnvalue))
  (`UserWidget.AddToViewport` _output_get 0))

(event `DialougeVisibility`
  (`CharacterMovementComponent.SetMovementMode` (`self.CharacterMovement`) "MOVE_Walking" 0)
  (`Widget.SetVisibility` (`/Game/Blueprints/Dialouge/BP_PlayerDialogue.SpeechBubble` (`self.PlayerHUD`)) "Hidden"))

(event `InputAction|Speaking`
  (params (Key :type "Key Structure"))
  (:`Pressed`
    (`self.InteractTrace`)))

(event `/Game/Blueprints/Player_BI.Speaking`
  (params (Dialogue :type String) (TextDelay :type "Float (double-precision)"))
  (`/Game/Blueprints/Dialouge/BP_PlayerDialogue.INCSpeech` (`self.PlayerHUD`) Dialogue TextDelay))

(event `DamageableInterface.OnDeath`
  (bind _returnvalue (`GameplayStatics.GetActorOfClass` "/Game/Blueprints/BP_DayCycleManager.BP_DayCycleManager_C"))
  (`/Engine/EditorBlueprintResources/StandardMacros.IsValid` _returnvalue
    (:`Is Valid`
      (bind _returnvalue_2 (`DayCycleManager.GetPlayerSpawnLocation` _returnvalue))
      (`self.K2_SetActorLocation` _returnvalue_2)
      (`AttributeComponent.SetMaxHealth` (`self.GetComponentByClass` self "/Script/Cupcake.AttributeComponent") 100.0))
    (:`Is Not Valid`
      (`KismetSystemLibrary.PrintString` "No DNC actor in scene"))))

(event `DamageableInterface.OnDamage`
  (`SkeletalMeshComponent.PlayAnimation` (`self.Mesh`) "/Game/Player/Animations/HurtRough.HurtRough" false)
  (`KismetSystemLibrary.Delay` 0.666)
  (`SkeletalMeshComponent.SetAnimationMode` (`self.Mesh`) "AnimationBlueprint" true))

(event `self.DoAttack`
  (bind _mesh (`self.Mesh`))
  (if (not (`self.Attacking`))
    (set `self.Attacking` true)
    (`SkeletalMeshComponent.PlayAnimation` _mesh "/Game/Player/Animations/Punch.Punch" false)
    (`|PlayMontage` _mesh "/Game/Player/Animations/Punch_Montage.Punch_Montage"
      (:`then`
        (`KismetSystemLibrary.Delay` 1.1334 :!label _label)
        (`SkeletalMeshComponent.SetAnimationMode` (`self.Mesh`) "AnimationBlueprint" true)
        (set `self.Attacking` false))
      (:`OnCompleted`
        (goto _label))
      (:`OnNotifyBegin`
        (`FMODBlueprintStatics.PlayEvent2D` "/Game/FMOD/Events/AxeSwings.AxeSwings")))))

(fn `CheckSpeaking`
  (returns (bSpeaking :type Boolean))
  (return (`/Game/Blueprints/Dialouge/BP_PlayerDialogue.Looping` (`self.PlayerHUD`))))

(fn `InteractTrace`
  (bind _returnvalue (`SceneComponent.K2_GetComponentLocation` (`self.Scene`)))
  (bind (_outhit _returnvalue_2) (`KismetSystemLibrary.SphereTraceSingle` _returnvalue (- _returnvalue (0.0 0.0 90.0)) 45.0 "TraceTypeQuery1"))
  (if _returnvalue_2
    (bind _returnvalue_3 (`self.GetComponentByClass` (`.HitActor` (`GameplayStatics.BreakHitResult` _outhit)) "/Game/Blueprints/Dialouge/BC_Dialogue.BC_Dialogue_C"))
    (`/Engine/EditorBlueprintResources/StandardMacros.IsValid` _returnvalue_3
      (:`Is Valid`
        (`CharacterMovementComponent.SetMovementMode` (`self.CharacterMovement`) "MOVE_None" 0)
        (`/Game/Blueprints/Dialouge/BC_Dialogue.Speaking` _returnvalue_3)))))

(fn `UserConstructionScript`
  (`parent.UserConstructionScript`))