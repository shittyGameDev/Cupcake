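; Choppable tree actor that drops an item when it dies.
; OnDeath passes the player's CupcakeCharacter to the Drop component's DropItem, prints a debug message and destroys the tree.
; SpawnLeafParticle spawns an auto-released pooled Niagara leaf burst at the tree and plays a 2D chop sound.
; A RandomVector helper builds random XY offsets but is not called within this Blueprint.
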(event `self.ReceiveBeginPlay`)

(event `DamageableInterface.OnDeath`
  (bind _ascupcake_character (cast `CupcakeCharacter` (`GameplayStatics.GetPlayerCharacter` 0)))
  (`DropComponent.DropItem` (`self.Drop`) _ascupcake_character)
  (`KismetSystemLibrary.PrintString` "Done")
  (`self.K2_DestroyActor`))

(event `self.SpawnLeafParticle`
  (`NiagaraFunctionLibrary.SpawnSystemAtLocation` "/Game/VFX/Enviroment/NS_Leaves.NS_Leaves" (`self.K2_GetActorLocation`) (struct) (1.0 1.0 1.0) true true "AutoRelease")
  (`GameplayStatics.PlaySound2D` "/Game/TempSounds/442534__super8ude__treechop3.442534__super8ude__treechop3" 0.3 1.0 0.0 null null false))

(fn `Random Vector`
  (params (Min :type "Float (double-precision)") (Max :type "Float (double-precision)"))
  (returns (`Return Value` :type "Vector Structure"))
  (return (`KismetMathLibrary.MakeVector` (`KismetMathLibrary.RandomFloatInRange` Min Max) (`KismetMathLibrary.RandomFloatInRange` Min Max))))

(fn `UserConstructionScript`)