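; BP_TreeHandWeapon is a tree enemy's hand weapon that knocks the player back when they overlap it.
; On overlap it disables the player's movement, constrains the capsule to the XY plane and briefly switches it to physics simulation.
; A horizontal velocity-change impulse, scaled by Force along the direction away from the weapon, launches the player.
; After a short delay it turns physics off and restores walking.
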(event `self.ReceiveActorBeginOverlap`
  (params (OtherActor :type "Actor Object Reference"))
  (bind _player (`self.Player`))
  (bind _asbp_player_character (cast `/Game/Player/BP_PlayerCharacter` OtherActor))
  (bind _output_get (set `self.Player` _asbp_player_character))
  (`CharacterMovementComponent.SetMovementMode` (`Character.CharacterMovement` _output_get) "MOVE_None" 0)
  (bind _capsulecomponent (`Character.CapsuleComponent` _output_get))
  (`PrimitiveComponent.SetConstraintMode` _capsulecomponent "XYPlane")
  (`KismetSystemLibrary.Delay` 0.05)
  (`PrimitiveComponent.SetSimulatePhysics` _capsulecomponent true)
  (`PrimitiveComponent.AddImpulse` _capsulecomponent (`KismetMathLibrary.MakeVector` (.x (* (`KismetMathLibrary.Normal` (- (`self.K2_GetActorLocation` (`GameplayStatics.GetPlayerPawn` 0)) (`self.K2_GetActorLocation`))) (`self.Force`))) (.y (* (`KismetMathLibrary.Normal` (- (`self.K2_GetActorLocation` (`GameplayStatics.GetPlayerPawn` 0)) (`self.K2_GetActorLocation`))) (`self.Force`)))) "None" true)
  (`KismetSystemLibrary.Delay` 1.0)
  (`PrimitiveComponent.SetSimulatePhysics` (`Character.CapsuleComponent` _player) false)
  (`PrimitiveComponent.SetConstraintMode` _capsulecomponent "None")
  (`CharacterMovementComponent.SetMovementMode` (`Character.CharacterMovement` _player) "MOVE_Walking" 0))

(fn `UserConstructionScript`)