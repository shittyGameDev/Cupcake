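; BlockingActor1 is a trigger actor that removes a BP_BigStone from the level when the player overlaps it.
; Both begin and end overlap share one path that compares OtherActor to ABP_Player.
; On a match, it destroys the BP_BigStone returned by GetActorOfClass, without a linked reference or validity check.
; Cast-based destroy chains using a Stone reference are left disconnected, and construction is empty.
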(event `self.ReceiveActorEndOverlap`
  (params (OtherActor :type "Actor Object Reference"))
  (if (== (stale `self.ReceiveActorBeginOverlap` OtherActor) "/Game/Player/ABP_Player.ABP_Player") :!label _label
    (bind _returnvalue (`GameplayStatics.GetActorOfClass` "/Game/Blueprints/BP_BigStone.BP_BigStone_C"))
    (`self.K2_DestroyActor` _returnvalue)))

(event `self.ReceiveActorBeginOverlap`
  (params (OtherActor :type "Actor Object Reference"))
  (goto _label))

(fn `UserConstructionScript`)