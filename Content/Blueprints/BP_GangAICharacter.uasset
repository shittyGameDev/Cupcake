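; Gang AI character Blueprint that sets its max health through an AttributeComponent and drops mushroom loot when it dies.
; On death, a custom while-loop macro spawns MushroomDrop actors at random horizontal offsets around the character, then destroys its weapon and itself.
; The loop runs while a counter is below a random integer drawn from LootAmount, so the drop count varies.
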(event `self.ReceiveBeginPlay`
  (`AttributeComponent.SetMaxHealth` (`self.GetComponentByClass` self "/Script/Cupcake.AttributeComponent") 100.0))

(event `DamageableInterface.OnDeath`
  (while (< (`self.Counter`) (`KismetMathLibrary.RandomInteger` (`self.LootAmount`))) :!label _label
    (`|SpawnActorFromClass` "/Game/Blueprints/ItemFolder/MushroomDrop.MushroomDrop_C" (`KismetMathLibrary.Conv_VectorToTransform` (+ (.location (`self.GetTransform`)) (`self.Random Vector` -200.0 200.0))) "Undefined" "MultiplyWithRoot" null null)
    (set `self.Counter` (+ 1 (`self.Counter`)))
    (goto _label))
  (`self.K2_DestroyActor` (`self.Weapon`))
  (`self.K2_DestroyActor`))

(fn `Random Vector`
  (params (Min :type "Float (double-precision)") (Max :type "Float (double-precision)"))
  (returns (`Return Value` :type "Vector Structure"))
  (return (`KismetMathLibrary.MakeVector` (`KismetMathLibrary.RandomFloatInRange` Min Max) (`KismetMathLibrary.RandomFloatInRange` Min Max))))

(fn `UserConstructionScript`)