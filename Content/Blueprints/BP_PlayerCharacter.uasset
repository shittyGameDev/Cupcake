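; Player character Blueprint that lets the player trigger dialogue on nearby actors and shows the speech on screen.
; BeginPlay creates the BP_PlayerDialogue HUD widget.
; The Speaking input runs a debug-drawn, downward sphere trace from a scene component and calls Speaking on the hit actor's BC_Dialogue component.
; A Speaking event forwards text and delay to the HUD, while CheckSpeaking returns the HUD's Looping state.
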(event `self.ReceiveBeginPlay`
  (`parent.ReceiveBeginPlay`)
  (bind _returnvalue (`|CreateWidget` "/Game/Blueprints/Dialouge/BP_PlayerDialogue.BP_PlayerDialogue_C"))
  (bind _output_get (set `self.PlayerHUD` _returnvalue))
  (`UserWidget.AddToViewport` _output_get 0))

(event `InputAction|Speaking`
  (params (Key :type "Key Structure"))
  (:`Pressed`
    (`self.InteractTrace`)))

(event `/Game/Blueprints/Player_BI.Speaking`
  (params (Dialogue :type String) (TextDelay :type "Float (double-precision)"))
  (`/Game/Blueprints/Dialouge/BP_PlayerDialogue.INCSpeech` (`self.PlayerHUD`) Dialogue TextDelay))

(fn `CheckSpeaking`
  (returns (bSpeaking :type Boolean))
  (return (`/Game/Blueprints/Dialouge/BP_PlayerDialogue.Looping` (`self.PlayerHUD`))))

(fn `InteractTrace`
  (bind _returnvalue (`SceneComponent.K2_GetComponentLocation` (`self.Scene`)))
  (bind (_outhit _returnvalue_2) (`KismetSystemLibrary.SphereTraceSingle` :`Start` _returnvalue :`End` (- _returnvalue (0.0 0.0 90.0)) :`Radius` 45.0 :`TraceChannel` "TraceTypeQuery1" :`DrawDebugType` "ForDuration"))
  (if _returnvalue_2
    (bind _returnvalue_3 (`self.GetComponentByClass` (`.HitActor` (`GameplayStatics.BreakHitResult` _outhit)) "/Game/Blueprints/Dialouge/BC_Dialogue.BC_Dialogue_C"))
    (`/Engine/EditorBlueprintResources/StandardMacros.IsValid` _returnvalue_3
      (:`Is Valid`
        (`/Game/Blueprints/Dialouge/BC_Dialogue.Speaking` _returnvalue_3)))))

(fn `UserConstructionScript`
  (`parent.UserConstructionScript`))